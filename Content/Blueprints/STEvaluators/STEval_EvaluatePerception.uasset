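; State Tree evaluator that turns an enemy AI controller's perception updates into stimulus and sight state.
; It binds to the controller's AIPerception on tree start and unbinds on stop.
; Successful stimuli record the perceived actor, and sight stimuli also set CanSeeTarget; nothing resets these flags.
; Target acquisition, which would set focus and Attack motivation through a property reference, is never called, and the forgotten handler is empty.
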(event `self.ReceiveTreeStart`
  (bind _aiperception (`/Game/Blueprints/AIC_NPC_Enemy.AIPerception` (`self.Enemy AIC Ref`)))
  (add `AIPerceptionComponent.OnTargetPerceptionUpdated` _aiperception (`|CreateDelegate` :!event `OnTargetPerceptionUpdated`))
  (add `AIPerceptionComponent.OnTargetPerceptionForgotten` _aiperception (`|CreateDelegate` :!event `OnTargetPerseptionForgotten`)))

(event `self.ReceiveTreeStop`
  (bind _aiperception (`/Game/Blueprints/AIC_NPC_Enemy.AIPerception` (`self.Enemy AIC Ref`)))
  (remove `AIPerceptionComponent.OnTargetPerceptionUpdated` _aiperception (`|CreateDelegate` :!event `OnTargetPerceptionUpdated`))
  (remove `AIPerceptionComponent.OnTargetPerceptionForgotten` _aiperception (`|CreateDelegate` :!event `OnTargetPerseptionForgotten`)))

(event `OnTargetPerceptionUpdated`
  (params (Actor :type "Actor Object Reference") (Stimulus :type "AIStimulus Structure"))
  (set `self.Perceibed Actor` Actor)
  (bind _output_get (set `self.Received Stimulus` Stimulus))
  (if (`.bSuccessfullySensed` (break `AIStimulus` _output_get))
    (set `self.ReceivedAnyStimulus` true)
    (`self.HandleSightStimulus`)
    (`KismetSystemLibrary.PrintString` (`KismetSystemLibrary.GetDisplayName` (`self.Acquired Target`)))))

(event `OnTargetPerseptionForgotten`
  (params (Actor :type "Actor Object Reference")))

(fn `HandleSightStimulus`
  (bind _returnvalue (`AIPerceptionSystem.GetSenseClassForStimulus` (`self.Received Stimulus`)))
  (if (and (== _returnvalue "/Script/AIModule.AISense_Sight") (`self.ReceivedAnyStimulus`))
    (set `self.Received Sight Stimulus` true)
    (if (`.bSuccessfullySensed` (break `AIStimulus` (`self.Received Stimulus`)))
      (set `self.Can See target` true))))

(fn `Set Acquired Target`
  (bind _acquired_target (`self.Acquired Target`)
    (:`then`
      (if (not (== _acquired_target (`self.Perceibed Actor`)))
        (set `self.Acquired Target` (`self.Perceibed Actor`) :!label _label)))
    (:`else`
      (goto _label)))
  (`AIController.K2_SetFocus` (`self.Enemy AIC Ref`) (`self.Acquired Target`))
  (bind _reference (`|StateTreeBlueprintPropertyRef` (`self.Motivation Param`))
    (:`Succeeded`
      (`|VariableSetRef` _reference (struct :`TagName` "Enemy.Motivation.Attack"))
      (return))
    (:`Failed`
      (return))))