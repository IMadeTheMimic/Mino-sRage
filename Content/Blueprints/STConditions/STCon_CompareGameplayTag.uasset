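; A StateTree condition Blueprint that tests whether one gameplay tag matches another.
; The test passes LeftTag and RightTag to MatchesTag, with an ExactMatch flag choosing between exact and hierarchical matching.
; A custom description shows the left tag's binding, the match type and the right tag's name.
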(fn `Get`)

(fn `ReceiveGetDescription`
  (params (Formatting :type "EStateTreeNodeFormatting Enum" :default "RichText"))
  (returns (ReturnValue :type Text))
  (return (`|FormatText` "Tag[{Left}]{Operator}{Right}" (`|GenericToText` (`self.BindingDescription`)) (`KismetMathLibrary.SelectText` "Is exact match" "Is Match" (`self.Exact Match`)) (`|GenericToText` (`BlueprintGameplayTagLibrary.GetTagName` (`self.RightTag`))))))

(fn `ReceiveTestCondition`
  (returns (ReturnValue :type Boolean))
  (return (`BlueprintGameplayTagLibrary.MatchesTag` (`self.LeftTag`) (`self.RightTag`) (`self.Exact Match`))))